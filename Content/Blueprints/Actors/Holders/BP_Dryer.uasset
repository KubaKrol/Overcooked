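; BP_Dryer is a dryer holder actor that displays the progress of its interaction on a world-space progress bar.
; BeginPlay caches the WBP_ProgressBar instance from the widget component.
; Each tick it polls the Interactable component and shows the bar only while progress is strictly between zero and one.
; While visible, the bar updates its percent and rotates to face the player camera.
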(event EventBeginPlay
  (bind _aswbp_progress_bar (Utilities|Casting|CastToWBP_ProgressBar (UserInterface|GetWidget (Variables|Default|GetProgressBarWidget))))
  (Variables|Default|SetAs%20WBP%20Progress%20Bar _aswbp_progress_bar))

(event EventTick
  (params (DeltaSeconds :type Float%20%28single-precision%29))
  (bind _interactable (Variables|Default|GetInteractable))
  (bind _returnvalue (Class|InteractableComponent|GetInteractionProgress _interactable))
  (bind _returnvalue_2 (> _returnvalue 0.0))
  (bind _returnvalue_3 (< _returnvalue 1.0))
  (bind _returnvalue_4 (and _returnvalue_3 _returnvalue_2))
  (Rendering|SetVisibility (Variables|Default|GetProgressBarWidget) _returnvalue_4 false)
  (if _returnvalue_4
    (Progress|SetPercent (Variables|/Game/Blueprints/UI/WBP_ProgressBar.WBP_ProgressBar_C|GetProgressBar (Variables|Default|GetAs%20WBP%20Progress%20Bar)) (Class|InteractableComponent|GetInteractionProgress (Variables|Default|GetInteractable)))
    (Transformation|SetWorldRotation (Variables|Default|GetProgressBarWidget) (Math|Rotator|FindLookatRotation (Transformation|GetWorldLocation (Variables|Default|GetProgressBarWidget)) (Camera|GetCameraLocation (Game|GetPlayerCameraManager 0))) false false)))

(fn ConstructionScript)