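; BP_Washer is a holder station that runs a quick time event to wash a held Client.
; Initializing with Shampoo queues two button presses and a movement wiggle on the QuickTimeEvent component.
; While it runs, Tick shows camera-facing world widgets for progress and the current action name.
; On finish, the held Client's task index is incremented; the plain initialize and per-action handlers are empty.
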(event Custom|OnInitialize_Event)

(event Custom|OnActionFinished_Event
  (params (ActionIndex :type Integer))
  (switch int ActionIndex))

(event Custom|OnInitializeWithHoldable_Event
  (params (HoldableName :type String))
  (bind _quicktimeevent (Variables|Default|GetQuickTimeEvent))
  (switch string HoldableName
    (:Shampoo
      (Class|QuickTimeEventComponent|AddPressAction _quicktimeevent "/Game/Input/Actions/IA_Player_Throw.IA_Player_Throw" "Press Triangle")
      (Class|QuickTimeEventComponent|AddPressAction _quicktimeevent "/Game/Input/Actions/IA_Player_SecondaryAction.IA_Player_SecondaryAction" "Press Square")
      (Class|QuickTimeEventComponent|AddWiggleAction _quicktimeevent "/Game/Input/Actions/IA_Player_Movement.IA_Player_Movement" 30 "Wiggle"))))

(event Custom|OnFinished_Event
  (bind _holder (Variables|Default|GetHolder))
  (if (Class|HolderComponent|IsHolding _holder)
    (bind _asclient (Utilities|Casting|CastToClient (Components|GetOwner (Class|HolderComponent|GetHoldableComponent _holder))))
    (Development|PrintString "Hello")
    (Class|Client|IncrementClientTaskIndex _asclient)))

(event EventBeginPlay
  (bind _quicktimeevent (Variables|Default|GetQuickTimeEvent))
  (EventDispatchers|AssignOnInitialize _quicktimeevent (delegate Custom|OnInitialize_Event))
  (EventDispatchers|AssignOnInitializewithHoldable _quicktimeevent (delegate Custom|OnInitializeWithHoldable_Event))
  (EventDispatchers|AssignOnActionFinished (Variables|Default|GetQuickTimeEvent) (delegate Custom|OnActionFinished_Event))
  (EventDispatchers|AssignOnFinished (Variables|Default|GetQuickTimeEvent) (delegate Custom|OnFinished_Event))
  (bind _aswbp_progress_bar (Utilities|Casting|CastToWBP_ProgressBar (UserInterface|GetWidget (Variables|Default|GetProgressBarWidget))))
  (Variables|Default|SetAs%20WBP%20Progress%20Bar _aswbp_progress_bar)
  (bind _aswbp_input_tip (Utilities|Casting|CastToWBP_InputTip (UserInterface|GetWidget (Variables|Default|GetInputTipWidget))))
  (Variables|Default|SetAs%20WBP%20Input%20Tip _aswbp_input_tip))

(event EventTick
  (params (DeltaSeconds :type Float%20%28single-precision%29))
  (bind _returnvalue (Game|GetPlayerCameraManager 0))
  (bind _quicktimeevent (Variables|Default|GetQuickTimeEvent))
  (bind _returnvalue_2 (Class|QuickTimeEventComponent|IsRunning _quicktimeevent))
  (bind _returnvalue_3 (Camera|GetCameraLocation _returnvalue))
  (Rendering|SetVisibility (Variables|Default|GetProgressBarWidget) _returnvalue_2 false)
  (Rendering|SetVisibility (Variables|Default|GetInputTipWidget) _returnvalue_2 false)
  (if _returnvalue_2
    (Transformation|SetWorldRotation (Variables|Default|GetProgressBarWidget) (Math|Rotator|FindLookatRotation (Transformation|GetWorldLocation (Variables|Default|GetProgressBarWidget)) _returnvalue_3) false false)
    (Transformation|SetWorldRotation (Variables|Default|GetInputTipWidget) (Math|Rotator|FindLookatRotation (Transformation|GetWorldLocation (Variables|Default|GetInputTipWidget)) _returnvalue_3) false false)
    (Progress|SetPercent (Variables|/Game/Blueprints/UI/Widgets/WBP_ProgressBar.WBP_ProgressBar_C|GetProgressBar (Variables|Default|GetAs%20WBP%20Progress%20Bar)) (Class|QuickTimeEventComponent|GetProgress (Variables|Default|GetQuickTimeEvent)))
    (Rendering|Components|TextRender|SetText (Variables|/Game/Blueprints/UI/Widgets/WBP_InputTip.WBP_InputTip_C|GetTextField (Variables|Default|GetAs%20WBP%20Input%20Tip)) (Utilities|Text|ToText(String) (Class|QuickTimeEventComponent|GetCurrentActionName (Variables|Default|GetQuickTimeEvent))))))

(fn ConstructionScript)